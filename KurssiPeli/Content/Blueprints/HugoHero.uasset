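; HugoHero is the playable 2D flipbook character, moved left and right along world X by input axes, with a jump action.
; BeginPlay sets game-only input, and the Up and Down keys switch the sprite between larger and smaller scales.
; A/D, jump, attack and capsule hits on "Surface"-tagged actors all set the same HugoWalking flipbook.
; Attack has no other effect, and a JumpZVelocity setter is unconnected.
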(event OnComponentHit(CapsuleComponent)
  (params (HitComponent :type Primitive%20Component%20Object%20Reference) (OtherActor :type Actor%20Object%20Reference) (OtherComp :type Primitive%20Component%20Object%20Reference) (NormalImpulse :type Vector :default "0, 0, 0") (Hit :type Hit%20Result%20Structure%20%28by%20ref%29))
  (if (Actor|ActorHasTag OtherActor "Surface")
    (Sprite|SetFlipbook (Variables|Default|GetSprite) "/Game/Flipbooks/HugoWalking.HugoWalking")))

(event EventBeginPlay
  (Input|SetInputModeGameOnly (Game|GetPlayerController 0)))

(event Collision|EventActorBeginOverlap
  (params (OtherActor :type Actor%20Object%20Reference)))

(event EventTick
  (params (DeltaSeconds :type Float%20%28single-precision%29)))

(event Input|ActionEvents|InputActionjump
  (params (Key :type Key%20Structure :default "None"))
  (:Pressed
    (Sprite|SetFlipbook (Variables|Default|GetSprite) "/Game/Flipbooks/HugoWalking.HugoWalking")
    (Character|Jump)))

(event Input|ActionEvents|InputActionAttack
  (params (Key :type Key%20Structure :default "None"))
  ;[1 1 1] Turha
  (:Pressed
    (Sprite|SetFlipbook (Variables|Default|GetSprite) "/Game/Flipbooks/HugoWalking.HugoWalking"))
  (:Released
    (Sprite|SetFlipbook (Variables|Default|GetSprite) "/Game/Flipbooks/HugoWalking.HugoWalking")))

(event Input|AxisEvents|InputAxisMove_right
  (params (AxisValue :type Float%20%28single-precision%29))
  (Pawn|Input|AddMovementInput "1.000000, 0, 0" AxisValue false))

(event Input|AxisEvents|InputAxisMove_left
  (params (AxisValue :type Float%20%28single-precision%29))
  (Pawn|Input|AddMovementInput "-1.000000, 0, 0" AxisValue false))

(event Input|KeyboardEvents|A
  (params (Key :type Key%20Structure :default "None"))
  (bind _sprite (Variables|Default|GetSprite))
  (:Pressed
    (Sprite|SetFlipbook _sprite "/Game/Flipbooks/HugoWalking.HugoWalking"))
  (:Released
    (Sprite|SetFlipbook _sprite "/Game/Flipbooks/HugoWalking.HugoWalking")))

(event Input|KeyboardEvents|D
  (params (Key :type Key%20Structure :default "None"))
  (bind _sprite (Variables|Default|GetSprite))
  (:Pressed
    (Sprite|SetFlipbook _sprite "/Game/Flipbooks/HugoWalking.HugoWalking"))
  (:Released
    (Sprite|SetFlipbook _sprite "/Game/Flipbooks/HugoWalking.HugoWalking")))

(event Input|KeyboardEvents|Up
  (params (Key :type Key%20Structure :default "None"))
  (:Pressed
    (Transformation|SetRelativeScale3D (Variables|Default|GetSprite) "7.000000,7.000000,7.000000")))

(event Input|KeyboardEvents|Down
  (params (Key :type Key%20Structure :default "None"))
  (:Pressed
    (Transformation|SetRelativeScale3D (Variables|Default|GetSprite) "5.000000,5.000000,5.000000")))

(fn ConstructionScript)