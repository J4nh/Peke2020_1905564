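; JumpItem is a pickup that temporarily boosts Hugo's jump height when touched.
; On overlap it checks the other actor's name for Hugo, raises the player character's JumpZVelocity, waits a few seconds, then restores a fixed value.
; Other overlaps go to a respawn-trigger check, and both paths call ResetPosition after a short delay.
; Tick only forwards to the parent class.
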(event EventBeginPlay)

(event Collision|EventActorBeginOverlap
  (params (OtherActor :type Actor%20Object%20Reference))
  (bind _returnvalue (Utilities|GetObjectName OtherActor))
  (bind _returnvalue_2 (Game|GetPlayerCharacter 0))
  (bind _charactermovement (Variables|/Script/Engine.Character|GetCharacterMovement _returnvalue_2))
  ;[1 1 1] Check if JumpItem hit Hugo.
  (bind _hitresult (CallFunction|CheckHugoHit _returnvalue))
  (if _hitresult
    ;[1 1 1] If hit Hugo, change jump height for some time
    (Variables|/Script/Engine.CharacterMovementComponent|SetJumpZVelocity _charactermovement 1.2e+03)
    (Development|PrintString "Jump Boost")
    (Utilities|FlowControl|Delay 5.0)
    (Variables|/Script/Engine.CharacterMovementComponent|SetJumpZVelocity _charactermovement 8e+02)
    (else
      ;[1 1 1] If not Hugo, check if we hit respawn trigger
      (CallFunction|CheckRespawnHit _returnvalue)))
  ;[1 1 1] Wait until next JumpItem appears and reset JumpItem values
  (Utilities|FlowControl|Delay 1.0)
  (CallFunction|ResetPosition))

(event EventTick
  (params (DeltaSeconds :type Float%20%28single-precision%29))
  (|CallParentFunction 0.0))

(fn ConstructionScript)